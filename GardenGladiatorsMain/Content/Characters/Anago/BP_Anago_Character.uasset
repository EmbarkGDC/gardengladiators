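; Character Blueprint for Anago, an early scaffold for a water-ability character with swim dash, water attack and bubble shield.
; BeginPlay only prints an init message, and WaterAttack and BubbleShield only print activation messages.
; SwimDash adds an unscaled forward-vector impulse, and no connected graph calls any of the three abilities.
; Water meter, cost, timer, effect and input nodes sit disconnected, so none of that logic runs.
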(event `self.ReceiveBeginPlay`
  (`KismetSystemLibrary.PrintString` "Anago Character Initialized"))

(fn `BubbleShield`
  (`KismetSystemLibrary.PrintString` "Bubble Shield Activated!"))

(fn `SwimDash`
  (`PrimitiveComponent.AddImpulse` (`self.GetActorForwardVector`)))

(fn `UserConstructionScript`)

(fn `WaterAttack`
  (`KismetSystemLibrary.PrintString` "Water Attack Activated!"))