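; Score manager actor that keeps per-player scores and a high score for cut-based scoring.
; BeginPlay initializes it with zero players, so AddScore's index check fails unless it is reinitialized.
; AddScore applies a multiplier and Perfect, Good or Missed adjustment, overwriting rather than accumulating the stored score.
; The high-score check runs before that calculation, and GetPlayerScore's inverted index test returns zero for non-negative indices.
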(event `self.ReceiveBeginPlay`
  (`self.InitializeScoreManager` 0))

(fn `AddScore`
  (params (PlayerIndex :type Integer) (ScoreToAdd :type Integer) (EScoreType :type "/Game/MyContent/EScoreType Enum" :default "NewEnumerator0"))
  (bind _returnvalue (* ScoreToAdd (`self.ScoreMultiplier`)))
  (`self.CheckAnd UpdateScore` PlayerIndex ScoreToAdd)
  (if (< PlayerIndex (`self.MaxPlayers`))
    (switch `/Game/MyContent/EScoreType` EScoreType
      (:`NewEnumerator0`
        (set `self.CalculatedScore` (`KismetMathLibrary.FTrunc` (+ _returnvalue (`self.PerfectCutBonus`)))))
      (:`NewEnumerator1`
        (set `self.CalculatedScore` (`KismetMathLibrary.FTrunc` (+ _returnvalue (`self.GoodCutBonus`)))))
      (:`NewEnumerator2`
        (set `self.CalculatedScore` (`KismetMathLibrary.FTrunc` (+ _returnvalue (`self.MissedCutPenalty`))))))
    (`KismetArrayLibrary.Array_Set` (`self.PlayerScores`) PlayerIndex (`self.CalculatedScore`))
    (`KismetSystemLibrary.PrintString` (`KismetStringLibrary.Conv_IntToString` (`self.CalculatedScore`)))))

(fn `CheckAnd UpdateScore`
  (params (PlayerIndex :type Integer) (PlayerScore :type Integer))
  (returns (NewHighScoreAchieved :type Integer))
  (`self.GetPlayerScore` PlayerIndex)
  (if (> (`self.Is Score`) (`self.CurrentHighScore`))
    (bind _output_get (set `self.CurrentHighScore` (`self.CalculatedScore`))))
  (return _output_get))

(fn `GetPlayerScore`
  (params (PlayerIndex :type Integer))
  (returns (Score :type Integer))
  (if (< PlayerIndex 0)
    (set `self.CurrentScore` (`|GetArrayItem` (`self.PlayerScores`) PlayerIndex))
    (else
      (set `self.CurrentScore` 0)))
  (return (`self.CurrentScore`)))

(fn `InitializeScoreManager`
  (params (NumPlayers :type Integer))
  (set `self.MaxPlayers` NumPlayers)
  (for _ (range NumPlayers)
    (`KismetArrayLibrary.Array_Add` (`self.PlayerScores`))
    (return))
  (return))

(fn `UserConstructionScript`)