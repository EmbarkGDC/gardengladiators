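; BP_BaseSushi is a base sushi actor that scores a player's strike as perfect, normal or missed.
; GetStrikeThreshold branches on two strike checks, whose graphs hold unwired range comparisons on the cutting board's CMValue.
; Each outcome adds to BP_TopDownChar's score, prints a message, calls LowerTheSushi on BP_SpiderWaiter and destroys the sushi.
; Box overlaps toggle SushiOverlap, and the Z key only prints a respawn message.
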(event `self.ReceiveBeginPlay`
  (`KismetSystemLibrary.Delay` 1.1)
  (set `self.SushiOverlap` false))

(event `Key|Z`
  (params (Key :type "Key Structure"))
  (:`Pressed`
    (`KismetSystemLibrary.PrintString` "Respawn Sushi")))

(event `self.Box.OnComponentBeginOverlap`
  (params (OverlappedComponent :type "PrimitiveComponent Object Reference") (OtherActor :type "Actor Object Reference") (OtherComp :type "PrimitiveComponent Object Reference") (OtherBodyIndex :type Integer) (bFromSweep :type Boolean) (SweepResult :type "HitResult Structure (by ref)"))
  (set `self.SushiOverlap` true)
  (`KismetSystemLibrary.PrintString` "Pick"))

(event `self.Box.OnComponentEndOverlap`
  (params (OverlappedComponent :type "PrimitiveComponent Object Reference") (OtherActor :type "Actor Object Reference") (OtherComp :type "PrimitiveComponent Object Reference") (OtherBodyIndex :type Integer))
  (set `self.SushiOverlap` false)
  (`KismetSystemLibrary.PrintString` "Up"))

(event `Get Strike Threshold`
  (bind _normalstrike_testsushi (`self.NormalStrike_TestSushi`))
  (bind _normalstrike_testsushi_2 (`self.NormalStrike_TestSushi`))
  (bind _perfectstrike_testsushi (`self.PerfectStrike_TestSushi`))
  (bind _strikemessage (`self.StrikeMessage`))
  (bind _cmvalue (`/Game/Blueprints/BP_CuttingBoard.CMValue` (`self.CuttingBoardRef`)))
  (bind _cmvalue_2 (`/Game/Blueprints/BP_CuttingBoard.CMValue` (`self.CuttingBoardRef`)))
  (bind _outactors (`GameplayStatics.GetAllActorsOfClass` "/Game/Blueprints/BP_CuttingBoard.BP_CuttingBoard_C"))
  (set `self.CuttingBoardRef` (`|GetArrayItem` _outactors))
  (if (and (>= _cmvalue_2 (`|GetArrayItem` _perfectstrike_testsushi)) (<= _cmvalue_2 (`|GetArrayItem` _perfectstrike_testsushi 1)))
    (bind _asbp_top_down_char (cast `/Game/Blueprints/BP_TopDownChar` (`GameplayStatics.GetPlayerCharacter` 0)))
    (bind _output_get (set `/Game/Blueprints/BP_TopDownChar.score` (+ (`self.PerfectScore`) (`/Game/Blueprints/BP_TopDownChar.score` _asbp_top_down_char)) _asbp_top_down_char))
    (set `self.Score_TestSushi` _output_get)
    (`KismetSystemLibrary.PrintString` (`|GetArrayItem` _strikemessage))
    (elif (or (and (>= _cmvalue (`|GetArrayItem` _normalstrike_testsushi)) (<= _cmvalue (`|GetArrayItem` _normalstrike_testsushi 1))) (and (>= _cmvalue (`|GetArrayItem` _normalstrike_testsushi_2 2)) (<= _cmvalue (`|GetArrayItem` _normalstrike_testsushi_2 3))))
      (bind _asbp_top_down_char_2 (cast `/Game/Blueprints/BP_TopDownChar` (`GameplayStatics.GetPlayerCharacter` 0)))
      (bind _output_get_2 (set `/Game/Blueprints/BP_TopDownChar.score` (+ (`self.NormalScore`) (`/Game/Blueprints/BP_TopDownChar.score` _asbp_top_down_char_2)) _asbp_top_down_char_2))
      (set `self.Score_TestSushi` _output_get_2)
      (`KismetSystemLibrary.PrintString` (`|GetArrayItem` _strikemessage 1))
      (else
        (bind _asbp_top_down_char_3 (cast `/Game/Blueprints/BP_TopDownChar` (`GameplayStatics.GetPlayerCharacter` 0)))
        (bind _output_get_3 (set `/Game/Blueprints/BP_TopDownChar.score` (+ (`self.MissedlScore`) (`/Game/Blueprints/BP_TopDownChar.score` _asbp_top_down_char_3)) _asbp_top_down_char_3))
        (set `self.Score_TestSushi` _output_get_3) ; Miss
        (`KismetSystemLibrary.PrintString` (`|GetArrayItem` _strikemessage 2)))))
  (bind _outactors_2 (`GameplayStatics.GetAllActorsOfClass` "/Game/Blueprints/BP_SpiderWaiter.BP_SpiderWaiter_C"))
  (set `self.Spawner` (`|GetArrayItem` _outactors_2))
  (`/Game/Blueprints/BP_SpiderWaiter.LowerTheSushi` (`self.Spawner`))
  (`self.K2_DestroyActor`))

(fn `UserConstructionScript`)