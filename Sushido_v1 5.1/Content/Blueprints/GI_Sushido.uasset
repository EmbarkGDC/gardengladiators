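; Game instance for Sushido that records the current character index for each of up to four players.
; CharacterIndex takes a player number and a character index, then branches on the player number to write the matching P1 to P4 variable.
; Player numbers are zero-based, and any value outside that range stores nothing.
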(fn `characterIndex`
  (params (PlayerCharacter :type Integer) (charIndex :type Integer))
  (if (== PlayerCharacter 0)
    (set `self.P1_currentCharacterIndex` charIndex)
    (elif (== PlayerCharacter 1)
      (set `self.P2_currentCharacterIndex` charIndex)
      (elif (== PlayerCharacter 2)
        (set `self.P3_currentCharacterIndex` charIndex)
        (elif (== PlayerCharacter 3)
          (set `self.P4_currentCharacterIndex` charIndex))))))