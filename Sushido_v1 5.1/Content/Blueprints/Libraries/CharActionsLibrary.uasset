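; Blueprint function library of character action helpers for player scoring and grab/cut state.
; AddScore and SubtractScore find a player character by index, cast it to BP_TopDownChar, then adjust and return its Score.
; SetCutting clears an IsGrab flag, while SetGrabbing sets a separately named IsGrabbing flag.
; All but SubtractScore print debug strings.
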(fn `AddScore`
  (params (PlayerNum :type Integer) (StrikeScore :type Integer))
  (returns (Score :type Integer))
  (bind _asbp_top_down_char (cast `/Game/Blueprints/BP_TopDownChar` (`GameplayStatics.GetPlayerCharacter` null PlayerNum)))
  (`KismetSystemLibrary.PrintString` null (`KismetStringLibrary.Conv_IntToString` StrikeScore))
  (bind _output_get (set `/Game/Blueprints/BP_TopDownChar.score` (+ (`/Game/Blueprints/BP_TopDownChar.score` _asbp_top_down_char) StrikeScore) _asbp_top_down_char))
  (return _output_get))

(fn `SetCutting`
  (returns (isGrabbing :type Boolean))
  (locals (isGrab :type Boolean))
  (`KismetSystemLibrary.PrintString` null "SetCutting")
  (if (`local.isGrab`)
    (bind _output_get (set `local.isGrab` false))
    (return _output_get)))

(fn `SetGrabbing`
  (locals (isGrabbing :type Boolean))
  (`KismetSystemLibrary.PrintString` null "SetGrabbing")
  (if (not (`local.isGrabbing`))
    (set `local.isGrabbing` true)))

(fn `SubtractScore`
  (params (PlayerNum :type Integer) (MIssScore :type Integer))
  (returns (Score :type Integer))
  (bind _asbp_top_down_char (cast `/Game/Blueprints/BP_TopDownChar` (`GameplayStatics.GetPlayerCharacter` null PlayerNum)))
  (bind _output_get (set `/Game/Blueprints/BP_TopDownChar.score` (- (`/Game/Blueprints/BP_TopDownChar.score` _asbp_top_down_char) MIssScore) _asbp_top_down_char))
  (return _output_get))