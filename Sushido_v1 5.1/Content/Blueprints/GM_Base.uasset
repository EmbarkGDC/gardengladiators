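; Base game mode for a local multiplayer top-down game, handling player joining, shared camera and game over.
; A gamepad button creates new players, while helper functions spawn and possess the character selected in GI_Sushido at a PlayerStart.
; Each tick centers every character's spring arm on the group's average location, scaling arm length by distance from it.
; Tick also swaps all widgets for W_GameOver once player 0 reaches MaxScore.
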(event `Key|Gamepad_Special_Left`
  (params (Key :type "Key Structure"))
  (:`Pressed`
    (`GameplayStatics.CreatePlayer` -1)))

(event `self.ReceiveTick`
  (params (DeltaSeconds :type "Float (single-precision)"))
  (bind _returnvalue (`GameplayStatics.GetPlayerController` 0))
  ;[0.1697 1 0] GameOver Function
  (`self.Camera System`)
  ;;[0 0.1624 1] Score Trigger(Replace with reference to score trigger)
  (bind _asbp_top_down_char (cast `/Game/Blueprints/BP_TopDownChar` (`GameplayStatics.GetPlayerCharacter` 0)))
  (if (>= (`/Game/Blueprints/BP_TopDownChar.score` _asbp_top_down_char) (`self.MaxScore`))
    (`/Engine/EditorBlueprintResources/StandardMacros.DoOnce` true :!label _label
      (:`Completed`
        (`|ExecutionSequence`
          (:`then_0`
            (`WidgetLayoutLibrary.RemoveAllWidgets`))
          (:`then_1`
            (bind _returnvalue_2 (`|CreateWidget` "/Game/MyContent/UI/W_GameOver.W_GameOver_C"))
            (`UserWidget.AddToViewport` _returnvalue_2 0)
            (set `PlayerController.bShowMouseCursor` true _returnvalue)
            (`WidgetBlueprintLibrary.SetInputMode_UIOnlyEx` _returnvalue _returnvalue_2)))))
    (else
      (goto _label :!via `Reset`))))

(event `Camera System`
  ;[0.5312 0 0] Camera System
  (bind _outactors (`GameplayStatics.GetAllActorsOfClass` "/Game/Blueprints/BP_TopDownChar_Base.BP_TopDownChar_Base_C"))
  (bind _returnvalue (`GameplayStatics.GetActorArrayAverageLocation` _outactors))
  (for (_array_element _array_index) _outactors
    (bind _output (`|GetArrayItem` _outactors _array_index))
    (bind _returnvalue_2 (`self.K2_GetActorLocation` _output))
    ;;[1 1 1] Tilt characters based on zoom level / camera position to maintain illusion
    (`self.K2_SetActorRotation` _array_element (`KismetMathLibrary.MakeRotator` (`KismetMathLibrary.FClamp` (/ (`KismetMathLibrary.Vector_Distance` (`self.K2_GetActorLocation` _array_element) _returnvalue_2) -30.0) -60.0 0.0)) false)
    ;;[1 1 1] Get controlled player distance from other players
    (bind _output_get (set `self.targetArmLength` (* (`KismetMathLibrary.Vector_Distance` _returnvalue _returnvalue_2) 1.9)))
    ;;[1 1 1] Adjust spring arm length and camera position to keep players in frame
    (if (< _output_get 600.0)
      (set `self.targetArmLength` 600.0))
    (bind _springarm (`/Game/Blueprints/BP_TopDownChar_Base.SpringArm` _output))
    (set `SpringArmComponent.TargetArmLength` (`self.targetArmLength`) _springarm)
    (`SceneComponent.K2_SetWorldLocation` _springarm _returnvalue false false)))

(fn `Sushido_FindPlayerStart`
  (returns (PlayerStartTransform :type "Transform Structure"))
  (bind _returnvalue (`GameplayStatics.GetActorOfClass` "/Script/Engine.PlayerStart"))
  (return (`self.GetTransform` _returnvalue)))

(fn `Sushido_SpawnPlayer`
  (params (PlayerController :type "PlayerController Object Reference"))
  (bind _asgi_sushido (cast `/Game/Blueprints/GI_Sushido` (`GameplayStatics.GetGameInstance`)))
  (bind _returnvalue (`|SpawnActorFromClass` (`/Game/Blueprints/GI_Sushido.CharactersSelected` _asgi_sushido) (`self.Sushido_FindPlayerStart`) "Undefined" "MultiplyWithRoot" null null))
  (`Controller.Possess` PlayerController _returnvalue))

(fn `UserConstructionScript`)