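; BP_FishManager is a manager Blueprint that tracks registered characters and handles grabbing and placing fish.
; GrabFish requires a free character and SushiOverlap, then disables mesh collision, enables physics simulation and attaches the fish to the sprite's SushiSocket.
; PlaceFish attaches using the cutting board's socket name without a specified parent, clearing only the character's grab flag.
; SwitchGraphic and SendScoreToManager are empty stubs.
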(fn `Grab Fish`
  (params (Character :type "/Game/Blueprints/BP_TopDownChar_Base Object Reference") (FishObject :type "/Game/Blueprints/BP_BaseSushi Object Reference"))
  (bind _fish_mesh (`/Game/Blueprints/BP_BaseSushi.Fish_mesh` FishObject))
  (if (not (`/Game/Blueprints/BP_TopDownChar_Base.isGrabbing` Character))
    (`KismetSystemLibrary.PrintString` "Point 1")
    (if (`/Game/Blueprints/BP_BaseSushi.SushiOverlap` FishObject)
      (`KismetSystemLibrary.PrintString` "point 2")
      (`PrimitiveComponent.SetCollisionEnabled` _fish_mesh "NoCollision")
      (`PrimitiveComponent.SetSimulatePhysics` _fish_mesh true)
      (`self.K2_AttachToComponent` FishObject (`PaperCharacter.Sprite` Character) "SushiSocket" "KeepWorld" "KeepWorld" "KeepWorld" true)
      (set `/Game/Blueprints/BP_TopDownChar_Base.isGrabbing` true Character)
      (set `/Game/Blueprints/BP_BaseSushi.IsGrabbed` true FishObject))
    (else
      (return))))

(fn `Place Fish`
  (params (Character :type "/Game/Blueprints/BP_TopDownChar_Base Object Reference") (FishObject :type "/Game/Blueprints/BP_BaseSushi Object Reference"))
  (if (and (`/Game/Blueprints/BP_TopDownChar_Base.isGrabbing` Character) (`/Game/Blueprints/BP_BaseSushi.IsGrabbed` FishObject))
    (`self.K2_AttachToComponent` FishObject null (`SceneComponent.GetAttachSocketName` (`/Game/Mesh/FishObjects/BP_TestCuttingBoard.Cuttingboard_Mesh` (`self.Cutting Board`))) "KeepRelative" "KeepRelative" "KeepRelative" true)
    (set `/Game/Blueprints/BP_TopDownChar_Base.isGrabbing` false Character)))

(fn `RegisterCharacter`
  (params (CharacterToRegister :type "/Game/Blueprints/BP_TopDownChar_Base Object Reference"))
  (if (not (`KismetArrayLibrary.Array_Contains` (`self.Characters`) CharacterToRegister))
    (`KismetArrayLibrary.Array_Add` (`self.Characters`) CharacterToRegister)))

(fn `SendScoreToManager`)

(fn `SwitchGraphic`)

(fn `UserConstructionScript`)