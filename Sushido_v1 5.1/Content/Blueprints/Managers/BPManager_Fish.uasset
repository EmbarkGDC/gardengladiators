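; Fish manager that handles a player grabbing, placing and cutting sushi fish.
; Grab attaches an overlapped fish to the player's sprite socket and flags both as grabbed.
; Place snaps it to the cutting board socket, hands over state and messages the board; a note reports the fish disappearing when attached.
; Cut ends the cut meter, adds the sushi's score to player 0, destroys the fish and removes the meter UI.
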(fn `Player_FishCut`
  (params (`Cutting Board` :type "/Game/Mesh/FishObjects/BP_TestCuttingBoard Object Reference") (Sushi :type "/Game/Blueprints/BP_BaseSushi Object Reference"))
  (if (and (`/Game/Mesh/FishObjects/BP_TestCuttingBoard.TestCuttingBoard_Overlap` `Cutting Board`) (`/Game/Mesh/FishObjects/BP_TestCuttingBoard.SushiPlaced` `Cutting Board`))
    (`|ExecutionSequence`
      (:`then_0`
        (set `/Game/Mesh/FishObjects/BP_TestCuttingBoard.SushiPlaced` false `Cutting Board`)
        (`/Game/Mesh/FishObjects/BP_TestCuttingBoard.CutMeterEnd` `Cutting Board`)
        (`/Game/Blueprints/BP_BaseSushi.Get Strike Threshold` Sushi))
      (:`then_1`
        (`/Game/Blueprints/Libraries/CharActionsLibrary.AddScore` 0 (`/Game/Blueprints/BP_BaseSushi.Score_TestSushi` Sushi))
        (`Actor.K2_DetachFromActor` Sushi "KeepRelative" "KeepRelative" "KeepRelative")
        (`Actor.K2_DestroyActor` Sushi)
        (`Widget.RemoveFromParent` (`/Game/Mesh/FishObjects/BP_TestCuttingBoard.CutMeterRef` `Cutting Board`)) ; Removes Cut Meter from UI
      ))
    (else
      (`KismetSystemLibrary.PrintString` null "No Cutting Board nearby"))))

(fn `Player_FishGrab`
  (params (Player :type "/Game/Blueprints/BP_TopDownChar_Base Object Reference") (Fishs :type "/Game/Blueprints/BP_BaseSushi Object Reference"))
  (bind _fish_mesh (`/Game/Blueprints/BP_BaseSushi.Fish_mesh` Fishs))
  (if (not (`/Game/Blueprints/BP_TopDownChar_Base.isGrabbing` Player))
    (`KismetSystemLibrary.PrintString` null "Point 1")
    (if (`/Game/Blueprints/BP_BaseSushi.SushiOverlap` Fishs)
      (`KismetSystemLibrary.PrintString` null "point 2")
      (`PrimitiveComponent.SetCollisionEnabled` _fish_mesh "NoCollision")
      (`PrimitiveComponent.SetSimulatePhysics` _fish_mesh true)
      (`Actor.K2_AttachToComponent` Fishs (`PaperCharacter.Sprite` Player) "SushiSocket" "KeepWorld" "KeepWorld" "KeepWorld" true)
      (set `/Game/Blueprints/BP_TopDownChar_Base.isGrabbing` true Player)
      (set `/Game/Blueprints/BP_BaseSushi.IsGrabbed` true Fishs)
      (else
        (`KismetSystemLibrary.PrintString` null "point 3")))
    (else
      (return))))

(fn `Player_FishPlace`
  (params (`Player Grab` :type "/Game/Blueprints/BP_TopDownChar_Base Object Reference") (`Fish Grab` :type "/Game/Blueprints/BP_BaseSushi Object Reference") (CuttingBoard :type "/Game/Mesh/FishObjects/BP_TestCuttingBoard Object Reference"))
  (if (and (`/Game/Blueprints/BP_TopDownChar_Base.isGrabbing` `Player Grab`) (`/Game/Blueprints/BP_BaseSushi.IsGrabbed` `Fish Grab`))
    (`Actor.K2_AttachToComponent` `Fish Grab` (`/Game/Mesh/FishObjects/BP_TestCuttingBoard.Cuttingboard_Mesh` CuttingBoard) "FishCutting" "SnapToTarget" "SnapToTarget" "SnapToTarget" true) ; When Fish is attatched, it dissapears. Possible Fix might be typing out socket name
    (set `/Game/Blueprints/BP_TopDownChar_Base.isGrabbing` false `Player Grab`)
    (set `/Game/Blueprints/BP_BaseSushi.IsGrabbed` false `Fish Grab`)
    (set `/Game/Mesh/FishObjects/BP_TestCuttingBoard.SushiPlaced` true CuttingBoard)
    (`KismetSystemLibrary.PrintString` null "Place Failed")
    (message `/Game/Blueprints/Interfaces/BPI_InteractionPlaceSushi.BPI_PlaceSushi` CuttingBoard)))