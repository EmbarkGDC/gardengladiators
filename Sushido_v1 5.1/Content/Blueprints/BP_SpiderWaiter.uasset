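; BP_SpiderWaiter is a flipbook-animated spider that lowers randomly chosen sushi into the level at random BP_SpawnPoint locations.
; It picks sushi by cumulative weighted Score, attaches it, teleports to a spawn point, descends, detaches it, then ascends using a reversed descend animation.
; The cycle runs on BeginPlay, and LowerTheSushi replays it, polling until the Ready flag is set.
; Older randomized spawn logic remains disconnected.
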(event `self.ReceiveEndPlay`
  (params (EndPlayReason :type "EEndPlayReason Enum" :default "Destroyed"))
  ; Get random spawn location for SpiderWaiter
  (`KismetArrayLibrary.Array_Clear` (`/Game/Blueprints/BP_SpawnLocations.spawnLocations` (`self.spawnLocation`))))

(event `GetSpawnLocations`
  ; Get random spawn location for SpiderWaiter
  (bind _outactors (`GameplayStatics.GetAllActorsOfClass` "/Game/Blueprints/BP_SpawnPoint.BP_SpawnPoint_C"))
  (for _array_element _outactors
    (`KismetArrayLibrary.Array_Add` (`/Game/Blueprints/BP_SpawnLocations.spawnLocations` (`self.spawnLocation`)) (`self.GetTransform` _array_element))))

(event `self.ReceiveBeginPlay`
  (bind _defaultsceneroot (`self.DefaultSceneRoot`))
  (bind _paperflipbook (`self.PaperFlipbook`))
  ; Spawn fish
  ;;[0 1 0.1244] Spawner Activated
  (`KismetSystemLibrary.Delay` 1.0 :!label _label)
  (set `self.ready` false)
  (set `self.TotalProbability` 0.0)
  ;; Choose which fish to spawn
  (`self.CalculateProbability`)
  (bind _sushi (`self.GrabItemToSpawn`))
  (bind _returnvalue (`|SpawnActorFromClass` (`.Sushi_6_B9678C1A458EBE35B9A126BF211F2EF2` (break `/Game/Blueprints/Structure/S_SushidoFish` _sushi)) (`KismetMathLibrary.Conv_VectorToTransform` (+ (+ (`SceneComponent.K2_GetComponentLocation` _defaultsceneroot) (`SceneComponent.K2_GetComponentRotation` _defaultsceneroot)) (0.0 -50.0 -100.0))) "Undefined" "MultiplyWithRoot" null null))
  ; Attach fish to spider waiter
  (`self.K2_AttachToActor` _returnvalue self "None" "KeepWorld" "KeepWorld" "KeepWorld" true)
  (`self.GetSpawnLocations`)
  ; Set SpiderWaiter and fish location to random spawn point
  (set `self.RandomSpawn` (`self.K2_GetActorLocation` (`KismetArrayLibrary.Array_Random` (stale `GetSpawnLocations` _outactors))))
  (`self.K2_SetActorLocation` (`self.RandomSpawn`))
  ; Move the spiderwaiter and fish down
  (`KismetSystemLibrary.MoveComponentTo` (`self.DefaultSceneRoot`) (+ (`SceneComponent.K2_GetComponentLocation` (`self.DefaultSceneRoot`)) (0.0 0.0 -180.0)) (struct) false false 0.7)
  ;[0.8281 0 0 0.5] Animation logic
  ;; Set animation to 'landing'
  (`PaperFlipbookComponent.SetFlipbook` _paperflipbook "/Game/Graphics/Sprites/NPC/Flipbooks/SpiderWaiter/SpiderWaiter_Land_px.SpiderWaiter_Land_px")
  ;; Detach fish from SpiderWaiter
  (`self.K2_DetachFromActor` _returnvalue "KeepWorld" "KeepWorld" "KeepWorld")
  (`PaperFlipbookComponent.SetLooping` _paperflipbook false)
  ;; Delay before starting ascend sequence
  (`KismetSystemLibrary.Delay` 0.7)
  (`PaperFlipbookComponent.SetLooping` _paperflipbook true)
  ;; Set anim to 'recoil'
  (`PaperFlipbookComponent.SetFlipbook` _paperflipbook "/Game/Graphics/Sprites/NPC/Flipbooks/SpiderWaiter/SpiderWaiter_Recoil_px.SpiderWaiter_Recoil_px")
  (`PaperFlipbookComponent.PlayFromStart` _paperflipbook)
  (`KismetSystemLibrary.Delay` 0.5)
  ;; Set anim to 'descend' but reverse playback for ascending
  (`PaperFlipbookComponent.SetFlipbook` _paperflipbook "/Game/Graphics/Sprites/NPC/Flipbooks/SpiderWaiter/SpiderWaiter_Descend_nx.SpiderWaiter_Descend_nx")
  (`PaperFlipbookComponent.ReverseFromEnd` _paperflipbook)
  ;; Ascend SpiderWaiter
  (`KismetSystemLibrary.MoveComponentTo` (`self.DefaultSceneRoot`) (+ (`SceneComponent.K2_GetComponentLocation` (`self.DefaultSceneRoot`)) (0.0 0.0 300.0)) (struct) false false 0.7)
  ;; Set anim back to 'descend'
  (`PaperFlipbookComponent.SetFlipbook` _paperflipbook "/Game/Graphics/Sprites/NPC/Flipbooks/SpiderWaiter/SpiderWaiter_Descend_px.SpiderWaiter_Descend_px")
  ;; Restart spawner
  (set `self.ready` true))

(event `LowerTheSushi`
  ; Spawn fish
  ;;[0 1 0.1244] Spawner Activated
  (if (`self.ready`) :!label _label_2
    (goto _label)
    (else
      (`KismetSystemLibrary.Delay` 0.5)
      (goto _label_2))))

(fn `CalculateProbability`
  ;[1 1 1] Calculate the total weight of the item (Probability)
  (for _array_element (`self.SushiItems`)
    (set `self.TotalProbability` (+ (`self.TotalProbability`) (`.Score_9_B66582EE42652EE0613D9F854FC713DF` (break `/Game/Blueprints/Structure/S_SushidoFish` _array_element))))))

(fn `GrabItemToSpawn`
  (returns (Sushi :type "/Game/Blueprints/Structure/S_SushidoFish Structure"))
  (locals (`Random Value` :type "Float (double-precision)" :default 0.0) (SelectedSushi :type "/Game/Blueprints/Structure/S_SushidoFish Structure"))
  ;[1 1 1] Grab sushi through the weighted (probability) system
  (set `local.Random Value` (`KismetMathLibrary.RandomFloatInRange` 0.0 (`self.TotalProbability`)))
  (for _array_element (`self.SushiItems`)
    (bind (_fishtype _fishtexture _sushitexture _fishmaterial _missscore _goodscore _perfscore _doesperfscoremult _score) (break `/Game/Blueprints/Structure/S_SushidoFish` _array_element))
    (if (<= (`local.Random Value`) _score)
      (set `local.SelectedSushi` _array_element)
      (break)
      (else
        (set `local.Random Value` (- (`local.Random Value`) _score)))))
  (return (`local.SelectedSushi`)))

(fn `UserConstructionScript`)