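; BP_Dynamic_Camera is a camera actor, apparently for local multiplayer, whose graph logic is currently disconnected, so BeginPlay and construction do nothing.
; One unused chain sets the first player's view target to this actor.
; A second shuffles PlayerStarts, creates missing local players, spawns and possesses a BP_TopDownChar for each, then points their controllers at this shared camera.
; No camera movement logic appears in these graphs.
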(event `self.ReceiveBeginPlay`)

(fn `UserConstructionScript`)