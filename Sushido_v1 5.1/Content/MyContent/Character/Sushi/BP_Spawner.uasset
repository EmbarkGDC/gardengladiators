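; Sushi spawner actor that spawns a weighted-random sushi near its root, then lowers and raises that root.
; CalculateProbability totals the SushiItems weights, and GrabItemToSpawn subtracts weights from a random roll to pick the class.
; The cycle runs after BeginPlay and again on LowerTheSushi, which polls until Ready so cycles wait their turn.
; An older hard-coded random spawn switch is left disconnected.
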(event `self.ReceiveBeginPlay`
  (bind _defaultsceneroot (`self.DefaultSceneRoot`))
  ;[0 1 0.1244] Spawner Activated
  (`KismetSystemLibrary.Delay` 1.0 :!label _label)
  (set `self.ready` false)
  (set `self.TotalProbability` 0.0)
  (`self.CalculateProbability`)
  (bind _sushi (`self.GrabItemToSpawn`))
  (`|SpawnActorFromClass` (`.Sushi_6_B9678C1A458EBE35B9A126BF211F2EF2` (break `/Game/MyContent/Structure/SushiStruc` _sushi)) (`KismetMathLibrary.Conv_VectorToTransform` (+ (+ (`SceneComponent.K2_GetComponentLocation` _defaultsceneroot) (`SceneComponent.K2_GetComponentRotation` _defaultsceneroot)) (0.0 -50.0 -100.0))) "Undefined" "MultiplyWithRoot" null null)
  (`KismetSystemLibrary.MoveComponentTo` (`self.DefaultSceneRoot`) (+ (`SceneComponent.K2_GetComponentLocation` (`self.DefaultSceneRoot`)) (0.0 0.0 -300.0)) (struct) false false 0.7)
  (`KismetSystemLibrary.Delay` 0.5)
  (`KismetSystemLibrary.MoveComponentTo` (`self.DefaultSceneRoot`) (+ (`SceneComponent.K2_GetComponentLocation` (`self.DefaultSceneRoot`)) (0.0 0.0 300.0)) (struct) false false 0.7)
  (set `self.ready` true))

(event `LowerTheSushi`
  ;[0 1 0.1244] Spawner Activated
  (if (`self.ready`) :!label _label_2
    (goto _label)
    (else
      (`KismetSystemLibrary.Delay` 0.5)
      (goto _label_2))))

(fn `CalculateProbability`
  ;[1 1 1] Calculate the total weight of the item (Probability)
  (for _array_element (`self.SushiItems`)
    (set `self.TotalProbability` (+ (`self.TotalProbability`) (`.Wait_5_B66582EE42652EE0613D9F854FC713DF` (break `/Game/MyContent/Structure/SushiStruc` _array_element))))))

(fn `GrabItemToSpawn`
  (returns (Sushi :type "/Game/MyContent/Structure/SushiStruc Structure"))
  (locals (`Random Value` :type "Float (double-precision)" :default 0.0) (SelectedSushi :type "/Game/MyContent/Structure/SushiStruc Structure"))
  ;[1 1 1] Grab sushi through the weighted (probability) system
  (set `local.Random Value` (`KismetMathLibrary.RandomFloatInRange` 0.0 (`self.TotalProbability`)))
  (for _array_element (`self.SushiItems`)
    (bind (_sushi _wait) (break `/Game/MyContent/Structure/SushiStruc` _array_element))
    (if (<= (`local.Random Value`) _wait)
      (set `local.SelectedSushi` _array_element)
      (break)
      (else
        (set `local.Random Value` (- (`local.Random Value`) _wait)))))
  (return (`local.SelectedSushi`)))

(fn `UserConstructionScript`)