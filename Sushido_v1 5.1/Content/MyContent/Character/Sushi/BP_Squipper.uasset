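; BP_Squipper is a striking actor in a sushi scoring mechanic that drops 300 units over 0.7 seconds when play begins.
; A Center overlap counts as a perfect strike and adds 30 to the player character's score, while either Edges overlap is a plain hit without points.
; Both outcomes call LowerTheSushi on the first BP_Spawner found, then destroy this actor.
; The overlap check is marked as a placeholder for a power bar.
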(event `self.ReceiveBeginPlay`
  (bind _defaultsceneroot (`self.DefaultSceneRoot`))
  (`KismetSystemLibrary.MoveComponentTo` _defaultsceneroot (+ (`SceneComponent.K2_GetComponentLocation` _defaultsceneroot) (0.0 0.0 -300.0)) (struct) false false 0.7))

(event `self.Center.OnComponentBeginOverlap`
  (params (OverlappedComponent :type "PrimitiveComponent Object Reference") (OtherActor :type "Actor Object Reference") (OtherComp :type "PrimitiveComponent Object Reference") (OtherBodyIndex :type Integer) (bFromSweep :type Boolean) (SweepResult :type "HitResult Structure (by ref)"))
  ;[0.1302 0.1302 0.1302] Overlap Condition (Replace with Power Bar)
  ;[1 0.9065 0.2874] Perfect Strike
  (bind _asbp_top_down_char_p_1 (cast `/Game/MyContent/Character/BP_TopDownChar_Base` (`GameplayStatics.GetPlayerCharacter` 0)))
  (set `/Game/MyContent/Character/BP_TopDownChar_Base.score` (+ 30 (`/Game/MyContent/Character/BP_TopDownChar_Base.score` _asbp_top_down_char_p_1)) _asbp_top_down_char_p_1)
  ;[0.2191 0.8801 1] Reset Spawner, Destroy Sushi
  (bind _outactors (`GameplayStatics.GetAllActorsOfClass` "/Game/MyContent/Character/Sushi/BP_Spawner.BP_Spawner_C" :!label _label))
  (set `self.Spawner` (`|GetArrayItem` _outactors))
  (`/Game/MyContent/Character/Sushi/BP_Spawner.LowerTheSushi` (`self.Spawner`))
  (`self.K2_DestroyActor`))

(event `self.Edges2.OnComponentBeginOverlap`
  (params (OverlappedComponent :type "PrimitiveComponent Object Reference") (OtherActor :type "Actor Object Reference") (OtherComp :type "PrimitiveComponent Object Reference") (OtherBodyIndex :type Integer) (bFromSweep :type Boolean) (SweepResult :type "HitResult Structure (by ref)"))
  ;[0.1302 0.1302 0.1302] Overlap Condition (Replace with Power Bar)
  ;[1 0.9671 0.9571] Hit
  (cast `/Game/MyContent/Character/BP_TopDownChar_Base` (`GameplayStatics.GetPlayerCharacter` 0) :!label _label_2)
  (goto _label))

(event `self.Edges1.OnComponentBeginOverlap`
  (params (OverlappedComponent :type "PrimitiveComponent Object Reference") (OtherActor :type "Actor Object Reference") (OtherComp :type "PrimitiveComponent Object Reference") (OtherBodyIndex :type Integer) (bFromSweep :type Boolean) (SweepResult :type "HitResult Structure (by ref)"))
  ;[0.1302 0.1302 0.1302] Overlap Condition (Replace with Power Bar)
  (goto _label_2))

(fn `UserConstructionScript`)