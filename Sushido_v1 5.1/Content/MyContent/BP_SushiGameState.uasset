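; Game state Blueprint for a sushi game, intended to track per-player scores in a PlayerScores array.
; It exposes functions to initialize, update and get scores by player index, with index validity checks in the latter two.
; The logic looks unfinished: initialization clears the array but its loop is empty, and the getter returns a constant zero.
; BeginPlay, Tick and the construction script do nothing.
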(fn `GetPlayerScore`
  (params (PlayerIndex :type Integer))
  (returns (Return :type Integer))
  (if (`KismetArrayLibrary.Array_IsValidIndex` :`IndexToTest` PlayerIndex)
    (set `self.PlayerScores` (`|MakeArray` PlayerIndex))
    (return 0)))

(fn `InitializePlayerScores`
  (params (NumPlayers :type Integer))
  (`KismetArrayLibrary.Array_Clear` (`self.PlayerScores`))
  (for _index (range NumPlayers 0)
    _))

(fn `UpdatePlayerScore`
  (params (PlayerIndex :type Integer) (ScoreToAdd :type Integer))
  (if (< (`KismetArrayLibrary.Array_IsValidIndex` (`self.PlayerScores`) PlayerIndex) 0)
    (set `self.PlayerScores` (`|MakeArray` ScoreToAdd))))

(fn `UserConstructionScript`)