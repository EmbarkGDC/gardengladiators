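; BP_Yellowtail is a yellowtail sushi target that awards points to the player when its hit zones are overlapped.
; A Center overlap counts as a perfect strike worth more points, while either edge overlap gives a smaller hit score, with no check on the overlapping actor.
; Each hit updates the player character's score, triggers the game mode's score popup, tells BP_SushiSpawn to lower the sushi, then destroys itself.
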(event `self.Center.OnComponentBeginOverlap`
  (params (OverlappedComponent :type "PrimitiveComponent Object Reference") (OtherActor :type "Actor Object Reference") (OtherComp :type "PrimitiveComponent Object Reference") (OtherBodyIndex :type Integer) (bFromSweep :type Boolean) (SweepResult :type "HitResult Structure (by ref)"))
  ;[0.1302 0.1302 0.1302] Overlap Condition (Replace with Power Bar)
  ;[1 0.9065 0.2874] Perfect Strike
  (bind _asbp_third_person_character_p1 (cast `/Game/ThirdPerson/Blueprints/BP_ThirdPersonCharacterP1` (`GameplayStatics.GetPlayerCharacter` 0)))
  (set `/Game/ThirdPerson/Blueprints/BP_ThirdPersonCharacterP1.Score` (+ 50 (`/Game/ThirdPerson/Blueprints/BP_ThirdPersonCharacterP1.Score` _asbp_third_person_character_p1)) _asbp_third_person_character_p1)
  ;[0.179 0.7812 0.3804] UI Popup
  (bind _outactors (`GameplayStatics.GetAllActorsOfClass` "/Game/ThirdPerson/Blueprints/BP_ThirdPersonGameMode.BP_ThirdPersonGameMode_C"))
  (bind _output_get (set `self.TheGame` (`|GetArrayItem` _outactors)))
  (set `/Game/ThirdPerson/Blueprints/BP_ThirdPersonGameMode.PlusScore` "+50" _output_get)
  (`/Game/ThirdPerson/Blueprints/BP_ThirdPersonGameMode.Score Change` (`self.TheGame`))
  ;[0.2191 0.8801 1] Reset Spawner, Destroy Sushi
  (bind _outactors_2 (`GameplayStatics.GetAllActorsOfClass` "/Game/CustomBlueprints/BP_SushiSpawn.BP_SushiSpawn_C" :!label _label))
  (set `self.Spawner` (`|GetArrayItem` _outactors_2))
  (`/Game/CustomBlueprints/BP_SushiSpawn.LowerTheSushi` (`self.Spawner`))
  (`self.K2_DestroyActor`))

(event `self.Edges2.OnComponentBeginOverlap`
  (params (OverlappedComponent :type "PrimitiveComponent Object Reference") (OtherActor :type "Actor Object Reference") (OtherComp :type "PrimitiveComponent Object Reference") (OtherBodyIndex :type Integer) (bFromSweep :type Boolean) (SweepResult :type "HitResult Structure (by ref)"))
  ;[0.1302 0.1302 0.1302] Overlap Condition (Replace with Power Bar)
  ;[1 0.9671 0.9571] Hit
  (bind _asbp_third_person_character_p1 (cast `/Game/ThirdPerson/Blueprints/BP_ThirdPersonCharacterP1` (`GameplayStatics.GetPlayerCharacter` 0) :!label _label_2))
  (set `/Game/ThirdPerson/Blueprints/BP_ThirdPersonCharacterP1.Score` (+ 5 (`/Game/ThirdPerson/Blueprints/BP_ThirdPersonCharacterP1.Score` _asbp_third_person_character_p1)) _asbp_third_person_character_p1)
  ;[0.179 0.7812 0.3804] UI Popup
  (bind _outactors (`GameplayStatics.GetAllActorsOfClass` "/Game/ThirdPerson/Blueprints/BP_ThirdPersonGameMode.BP_ThirdPersonGameMode_C"))
  (bind _output_get (set `self.TheGame` (`|GetArrayItem` _outactors)))
  (set `/Game/ThirdPerson/Blueprints/BP_ThirdPersonGameMode.PlusScore` "+5" _output_get)
  (`/Game/ThirdPerson/Blueprints/BP_ThirdPersonGameMode.Score Change` (`self.TheGame`))
  (goto _label))

(event `self.Edges1.OnComponentBeginOverlap`
  (params (OverlappedComponent :type "PrimitiveComponent Object Reference") (OtherActor :type "Actor Object Reference") (OtherComp :type "PrimitiveComponent Object Reference") (OtherBodyIndex :type Integer) (bFromSweep :type Boolean) (SweepResult :type "HitResult Structure (by ref)"))
  ;[0.1302 0.1302 0.1302] Overlap Condition (Replace with Power Bar)
  (goto _label_2))

(fn `UserConstructionScript`)