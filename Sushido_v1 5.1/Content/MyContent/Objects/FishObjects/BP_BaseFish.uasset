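; BP_BaseFish is a base fish actor for a sushi cutting game with pickup, placement and scored strikes.
; Box overlap fires an empty OnPickup if the player isn't grabbing; OnInteract attaches the fish to the player.
; GetStrikeThreshold adds perfect, normal or miss points to the player, calls LowerTheSushi on BP_SpiderWaiter, then destroys itself.
; Both strike checks leave their cutting board CMValue range comparisons unconnected, and IsInteractable returns false.
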(event `self.ReceiveBeginPlay`
  (`KismetSystemLibrary.Delay` 1.1)
  (set `self.SushiOverlap` false))

(event `self.Box.OnComponentBeginOverlap`
  (params (OverlappedComponent :type "PrimitiveComponent Object Reference") (OtherActor :type "Actor Object Reference") (OtherComp :type "PrimitiveComponent Object Reference") (OtherBodyIndex :type Integer) (bFromSweep :type Boolean) (SweepResult :type "HitResult Structure (by ref)"))
  (bind _asbp_top_down_char_base (cast `/Game/MyContent/Character/BP_TopDownChar_Base` OtherActor))
  (if true
    (`self.OnPlayerOverlap` _asbp_top_down_char_base)))

(event `OnPickup`
  (params (Character :type "/Game/MyContent/Character/BP_TopDownChar_Base Object Reference") (Fish :type "/Game/MyContent/Objects/FishObjects/BP_BaseFish Object Reference")))

(event `OnPlayerOverlap`
  (params (Character :type "/Game/MyContent/Character/BP_TopDownChar_Base Object Reference"))
  (bind _canbepickedup (`self.CanBePickedUp` Character))
  (if _canbepickedup
    (`self.OnPickup` Character)))

(event `/Game/MyContent/Objects/FishObjects/BPI_Interactable.OnInteract`
  (params (InteractingPlayer :type "Character Object Reference"))
  (`self.K2_AttachToActor` InteractingPlayer "None" "SnapToTarget" "SnapToTarget" "SnapToTarget")
  (`KismetSystemLibrary.PrintString` "Pick"))

(event `OnPlace`
  (params (RandNum :type Integer))
  (bind _output_get (set `self.FishPlaced` RandNum))
  (`KismetSystemLibrary.PrintString` (`KismetStringLibrary.Conv_IntToString` _output_get)))

(event `Get Strike Threshold`
  (bind _normalstrike_testsushi (`self.NormalStrike_TestSushi`))
  (bind _normalstrike_testsushi_2 (`self.NormalStrike_TestSushi`))
  (bind _perfectstrike_testsushi (`self.PerfectStrike_TestSushi`))
  (bind _strikemessage (`self.StrikeMessage`))
  (bind _cmvalue (`/Game/MyContent/Objects/FishObjects/BP_TestCuttingBoard.CMValue` (`self.CuttingBoardRef`)))
  (bind _cmvalue_2 (`/Game/MyContent/Objects/FishObjects/BP_TestCuttingBoard.CMValue` (`self.CuttingBoardRef`)))
  (bind _outactors (`GameplayStatics.GetAllActorsOfClass` "/Game/MyContent/Objects/FishObjects/BP_TestCuttingBoard.BP_TestCuttingBoard_C"))
  (set `self.CuttingBoardRef` (`|GetArrayItem` _outactors))
  (if (and (>= _cmvalue_2 (`|GetArrayItem` _perfectstrike_testsushi)) (<= _cmvalue_2 (`|GetArrayItem` _perfectstrike_testsushi 1)))
    (bind _asbp_top_down_char_base (cast `/Game/MyContent/Character/BP_TopDownChar_Base` (`GameplayStatics.GetPlayerCharacter` 0)))
    (bind _output_get (set `/Game/MyContent/Character/BP_TopDownChar_Base.score` (+ (`self.PerfectScore`) (`/Game/MyContent/Character/BP_TopDownChar_Base.score` _asbp_top_down_char_base)) _asbp_top_down_char_base))
    (set `self.Score_TestSushi` _output_get)
    (`KismetSystemLibrary.PrintString` (`|GetArrayItem` _strikemessage))
    (elif (or (and (>= _cmvalue (`|GetArrayItem` _normalstrike_testsushi)) (<= _cmvalue (`|GetArrayItem` _normalstrike_testsushi 1))) (and (>= _cmvalue (`|GetArrayItem` _normalstrike_testsushi_2 2)) (<= _cmvalue (`|GetArrayItem` _normalstrike_testsushi_2 3))))
      (bind _asbp_top_down_char_base_2 (cast `/Game/MyContent/Character/BP_TopDownChar_Base` (`GameplayStatics.GetPlayerCharacter` 0)))
      (bind _output_get_2 (set `/Game/MyContent/Character/BP_TopDownChar_Base.score` (+ (`self.NormalScore`) (`/Game/MyContent/Character/BP_TopDownChar_Base.score` _asbp_top_down_char_base_2)) _asbp_top_down_char_base_2))
      (set `self.Score_TestSushi` _output_get_2)
      (`KismetSystemLibrary.PrintString` (`|GetArrayItem` _strikemessage 1))
      (else
        (bind _asbp_top_down_char_base_3 (cast `/Game/MyContent/Character/BP_TopDownChar_Base` (`GameplayStatics.GetPlayerCharacter` 0)))
        (bind _output_get_3 (set `/Game/MyContent/Character/BP_TopDownChar_Base.score` (+ (`self.MissedlScore`) (`/Game/MyContent/Character/BP_TopDownChar_Base.score` _asbp_top_down_char_base_3)) _asbp_top_down_char_base_3))
        (set `self.Score_TestSushi` _output_get_3) ; Miss
        (`KismetSystemLibrary.PrintString` (`|GetArrayItem` _strikemessage 2)))))
  (bind _outactors_2 (`GameplayStatics.GetAllActorsOfClass` "/Game/MyContent/Character/Sushi/BP_SpiderWaiter.BP_SpiderWaiter_C"))
  (set `self.Spawner` (`|GetArrayItem` _outactors_2))
  (`/Game/MyContent/Character/Sushi/BP_SpiderWaiter.LowerTheSushi` (`self.Spawner`))
  (`self.K2_DestroyActor`))

(fn `CanBePickedUp`
  (params (Character :type "/Game/MyContent/Character/BP_TopDownChar_Base Object Reference"))
  (returns (CanBePickedUp :type Boolean))
  (if (`/Game/MyContent/Character/BP_TopDownChar_Base.isGrabbing` Character)
    (return false)
    (else
      (return true))))

(fn `IsInteractable`
  (returns (Interactable :type Boolean))
  (return false))

(fn `UserConstructionScript`)