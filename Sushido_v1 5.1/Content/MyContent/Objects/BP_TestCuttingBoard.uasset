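; Test cutting board actor that shows a place-sushi prompt on sphere overlap and runs a timing meter for cutting.
; An interface event hides the prompt, adds a W_CutMeter widget to the viewport and starts the meter.
; A retriggerable-delay loop, paced by PointerSpeed, bounces the value between 0 and 100 while SushiPlaced is true.
; CutMeterEnd prints the final value after a short delay and clears the cut-event flag.
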(event `self.ReceiveBeginPlay`)

(event `self.Sphere.OnComponentBeginOverlap`
  (params (OverlappedComponent :type "PrimitiveComponent Object Reference") (OtherActor :type "Actor Object Reference") (OtherComp :type "PrimitiveComponent Object Reference") (OtherBodyIndex :type Integer) (bFromSweep :type Boolean) (SweepResult :type "HitResult Structure (by ref)"))
  (`SceneComponent.SetVisibility` (`self.Widget_PlaceSushi`) true false)
  (set `self.TestCuttingBoard_Overlap` true))

(event `self.Sphere.OnComponentEndOverlap`
  (params (OverlappedComponent :type "PrimitiveComponent Object Reference") (OtherActor :type "Actor Object Reference") (OtherComp :type "PrimitiveComponent Object Reference") (OtherBodyIndex :type Integer))
  (`SceneComponent.SetVisibility` (`self.Widget_PlaceSushi`) false false)
  (set `self.TestCuttingBoard_Overlap` false))

(event `/Game/MyContent/Objects/BPI_InteractionPlaceSushi.BPI_PlaceSushi`
  (`KismetSystemLibrary.Delay` 0.2)
  (`KismetSystemLibrary.PrintString` "Prepare To CUT!")
  (`SceneComponent.SetVisibility` (`self.Widget_PlaceSushi`) false false)
  (bind _returnvalue (`|CreateWidget` "/Game/MyContent/UI/W_CutMeter.W_CutMeter_C"))
  (bind _output_get (set `self.CutMeterRef` _returnvalue))
  (cast `/Game/MyContent/UI/NewHUD` (`PlayerController.GetHUD` (`GameplayStatics.GetPlayerController` 0)))
  (`UserWidget.AddToViewport` _output_get 0)
  (`self.CutMeterStart`))

(event `CutMeterEnd`
  ;[0 0.1032 1] Prints Final Value of the Cut meter
  (`KismetSystemLibrary.Delay` 0.5)
  (`KismetSystemLibrary.PrintString` "Final Value")
  (`KismetSystemLibrary.PrintString` (`KismetStringLibrary.Conv_DoubleToString` (`self.CMValue`)))
  (set `self.CMEvent` false))

(event `CutMeterStart`
  (set `self.CMEvent` true)
  (set `self.CMValue` 0.0)
  (`KismetSystemLibrary.RetriggerableDelay` (`self.PointerSpeed`) :!label _label) ; Speed of the Pointer
  (if (`self.CMAdding`)
    (`self.CMAddValue`)
    (if (not (!= (`self.CMValue`) 100.0))
      (set `self.CMAdding` false))
    (else
      (`self.CMSubtractValue`)
      (if (not (!= (`self.CMValue`) 0.0))
        (set `self.CMAdding` true))))
  (if (`self.SushiPlaced`)
    (goto _label)))

(event `CMAddValue`
  ;[0 0.2401 1] CutMeterValue + 1.0
  (set `self.CMValue` (+ (`self.CMValue`) 1.0)))

(event `CMSubtractValue`
  ;[0 0.09324 1] CutMeterValue - 1.0
  (set `self.CMValue` (- (`self.CMValue`) 1.0)))

(fn `UserConstructionScript`)