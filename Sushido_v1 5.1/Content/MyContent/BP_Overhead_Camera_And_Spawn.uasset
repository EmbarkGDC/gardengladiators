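; BP_Overhead_Camera_And_Spawn sets up local multiplayer at BeginPlay and serves as the overhead camera shared by all players.
; It creates a local player with a controller for each PlayerStart index lacking one, using the array index as controller ID.
; The Characters array collects the existing BP_TopDownChar_p1 plus each CreatePlayer result.
; That array's indices then select each player controller whose view target switches to this actor.
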(event `self.ReceiveBeginPlay`
  (bind _returnvalue (`GameplayStatics.GetActorOfClass` "/Game/MyContent/Character/BP_TopDownChar_p1.BP_TopDownChar_p1_C"))
  (`KismetArrayLibrary.Array_Add` (`self.Characters`) _returnvalue)
  (bind _outactors (`GameplayStatics.GetAllActorsOfClass` "/Script/Engine.PlayerStart"))
  (bind _output_get (set `self.Spawn Points` _outactors))
  (for (_ _array_index) _output_get
    (bind _output_get_2 (set `self.Spawn Point Index` _array_index))
    (`/Engine/EditorBlueprintResources/StandardMacros.IsValid` (`GameplayStatics.GetPlayerController` _output_get_2)
      (:`Is Not Valid`
        (`GameplayStatics.CreatePlayer` (`self.Spawn Point Index`))
        (`KismetArrayLibrary.Array_Add` (`self.Characters`)))))
  (for (_ _array_index_2) (`self.Characters`)
    (`PlayerController.SetViewTargetWithBlend` (`GameplayStatics.GetPlayerController` _array_index_2) self 0.0 "VTBlend_Linear" 0.0 false)))

(fn `UserConstructionScript`)