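; Sushi spawner actor for the Sushido game that spawns one randomly picked actor at its root component's location and rotation.
; BeginPlay and the LowerTheSushi event both enter the same chain: a short delay, then a random integer switch.
; Switch outputs share five SpawnActor nodes unevenly, weighting the pick 5:4:3:1:1 out of fourteen.
; The chain has no loop, so another spawn needs LowerTheSushi to fire again.
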(event `LowerTheSushi`
  (bind _defaultsceneroot (`self.DefaultSceneRoot`))
  (bind _returnvalue (`KismetMathLibrary.Conv_VectorToTransform` (+ (`SceneComponent.K2_GetComponentLocation` _defaultsceneroot) (`SceneComponent.K2_GetComponentRotation` _defaultsceneroot))))
  ;[0 1 0.1244] Spawner Activated
  (`KismetSystemLibrary.Delay` 2.0 :!label _label)
  ;[0 1 0.85] Randomize Spawn
  (set `self.FSel` (`KismetMathLibrary.RandomInteger` 14))
  (switch `int` (`self.FSel`)
    (:`0`
      ;[1 0.8695 0] Spawn Actor
      (`|SpawnActorFromClass` null _returnvalue "Undefined" "MultiplyWithRoot" null null :!label _label_2))
    (:`1`
      (goto _label_2))
    (:`2`
      (goto _label_2))
    (:`3`
      (goto _label_2))
    (:`4`
      (goto _label_2))
    (:`5`
      (`|SpawnActorFromClass` null _returnvalue "Undefined" "MultiplyWithRoot" null null :!label _label_3))
    (:`6`
      (goto _label_3))
    (:`7`
      (goto _label_3))
    (:`8`
      (goto _label_3))
    (:`9`
      (`|SpawnActorFromClass` null _returnvalue "Undefined" "MultiplyWithRoot" null null :!label _label_4))
    (:`10`
      (goto _label_4))
    (:`11`
      (goto _label_4))
    (:`12`
      (`|SpawnActorFromClass` null _returnvalue "Undefined" "MultiplyWithRoot" null null))
    (:`13`
      (`|SpawnActorFromClass` null _returnvalue "Undefined" "MultiplyWithRoot" null null))))

(event `self.ReceiveBeginPlay`
  ;[0 1 0.1244] Spawner Activated
  (goto _label))

(fn `UserConstructionScript`)