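; Fish object (Heliouch) that scores the player's cutting strike as perfect, normal or missed.
; GetStrikeThreshold grabs the first BP_TestCuttingBoard, then branches on PerfectStrikeParam and NormalStrikeParam.
; Perfect doubles BP_TopDownChar's Score, normal leaves it unchanged, a miss subtracts points; each prints a message.
; Both Param graphs contain range comparisons on the board's CMValue, apparently not wired to an output.
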(event `Get Strike Threshold`
  (bind _normalstrike_testsushi (`self.NormalStrike_TestSushi`))
  (bind _normalstrike_testsushi_2 (`self.NormalStrike_TestSushi`))
  (bind _perfectstrike_testsushi (`self.PerfectStrike_TestSushi`))
  (bind _strikemessage (`self.StrikeMessage`))
  (bind _cmvalue (`/Game/Mesh/FishObjects/BP_TestCuttingBoard.CMValue` (`self.CuttingBoardRef`)))
  (bind _cmvalue_2 (`/Game/Mesh/FishObjects/BP_TestCuttingBoard.CMValue` (`self.CuttingBoardRef`)))
  (bind _outactors (`GameplayStatics.GetAllActorsOfClass` "/Game/Mesh/FishObjects/BP_TestCuttingBoard.BP_TestCuttingBoard_C"))
  (set `self.CuttingBoardRef` (`|GetArrayItem` _outactors))
  (if (and (>= _cmvalue_2 (`|GetArrayItem` _perfectstrike_testsushi)) (<= _cmvalue_2 (`|GetArrayItem` _perfectstrike_testsushi 1)))
    (bind _asbp_top_down_char (cast `/Game/Blueprints/BP_TopDownChar` (`GameplayStatics.GetPlayerCharacter` 0)))
    (bind _output_get (set `/Game/Blueprints/BP_TopDownChar.score` (* (`/Game/Blueprints/BP_TopDownChar.score` _asbp_top_down_char) 2) _asbp_top_down_char))
    (set `self.Score_TestSushi` _output_get)
    (`KismetSystemLibrary.PrintString` (`|GetArrayItem` _strikemessage))
    (elif (or (and (>= _cmvalue (`|GetArrayItem` _normalstrike_testsushi)) (<= _cmvalue (`|GetArrayItem` _normalstrike_testsushi 1))) (and (>= _cmvalue (`|GetArrayItem` _normalstrike_testsushi_2 2)) (<= _cmvalue (`|GetArrayItem` _normalstrike_testsushi_2 3))))
      (bind _asbp_top_down_char_2 (cast `/Game/Blueprints/BP_TopDownChar` (`GameplayStatics.GetPlayerCharacter` 0)))
      (bind _output_get_2 (set `/Game/Blueprints/BP_TopDownChar.score` (+ (`/Game/Blueprints/BP_TopDownChar.score` _asbp_top_down_char_2) 0) _asbp_top_down_char_2))
      (set `self.Score_TestSushi` _output_get_2)
      (`KismetSystemLibrary.PrintString` (`|GetArrayItem` _strikemessage 1))
      (else
        (bind _asbp_top_down_char_3 (cast `/Game/Blueprints/BP_TopDownChar` (`GameplayStatics.GetPlayerCharacter` 0)))
        (bind _output_get_3 (set `/Game/Blueprints/BP_TopDownChar.score` (+ (`/Game/Blueprints/BP_TopDownChar.score` _asbp_top_down_char_3) -50) _asbp_top_down_char_3))
        (set `self.Score_TestSushi` _output_get_3)
        (`KismetSystemLibrary.PrintString` (`|GetArrayItem` _strikemessage 2))))))

(fn `UserConstructionScript`)